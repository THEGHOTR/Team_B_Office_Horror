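; Door_BP is an interactable door that tracks locked and open state and supplies interaction prompts for the player.
; Interact clears the lock when locked, through a constant-true branch that leaves the "Door is Locked." message unreachable.
; When unlocked, a FlipFlop alternates the open flag and prints the result, with no door movement in these graphs.
; OpenPrompt and ClosePrompt write "Press E" text to the ThirdPersonCharacter's PlayerUI.
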(event `/Game/Logic/Interactables/InteractInterface.Interact`
  (if (`self.DoorLocked`)
    (cast `/Game/ThirdPersonBP/Blueprints/ThirdPersonCharacter` (`GameplayStatics.GetPlayerCharacter` 0))
    (if true
      (set `self.DoorLocked` false)
      (else
        (`KismetSystemLibrary.PrintString` "Door is Locked." true true (struct :`R` 1.0 :`G` 0.198 :`A` 1.0))))
    (else
      (`/Engine/EditorBlueprintResources/StandardMacros.FlipFlop`
        (:`A`
          (set `self.DoorOpen` true)
          (`KismetSystemLibrary.PrintString` "Door Opened" true true (struct :`G` 1.0 :`B` 0.016 :`A` 1.0)))
        (:`B`
          (set `self.DoorOpen` false)
          (`KismetSystemLibrary.PrintString` "Door Closed" true true (struct :`R` 1.0 :`B` 0.467875 :`A` 1.0)))))))

(event `Open Prompt`
  (bind _asthird_person_character (cast `/Game/ThirdPersonBP/Blueprints/ThirdPersonCharacter` (`GameplayStatics.GetPlayerCharacter` 0)))
  (set `/Game/UI/PlayerUI.InteractText` "Press E to Open" (`/Game/ThirdPersonBP/Blueprints/ThirdPersonCharacter.Player UI` _asthird_person_character)))

(event `Close Prompt`
  (bind _asthird_person_character (cast `/Game/ThirdPersonBP/Blueprints/ThirdPersonCharacter` (`GameplayStatics.GetPlayerCharacter` 0)))
  (set `/Game/UI/PlayerUI.InteractText` "Press E to Close" (`/Game/ThirdPersonBP/Blueprints/ThirdPersonCharacter.Player UI` _asthird_person_character)))

(fn `UserConstructionScript`)