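; Key_BP is a pickup key actor that marks the player as holding a key when interacted with.
; Interact destroys the actor, prints a pickup message and sets HasKey on the player's ThirdPersonCharacter.
; ShowPrompt and HidePrompt set and clear the pickup hint through InteractText on that character's PlayerUI.
; Leftover nodes for a key name on the GameMode and a text render are unconnected and never run.
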(event `self.ReceiveTick`
  (params (DeltaSeconds :type "Float (single-precision)")))

(event `/Game/Interactables/InteractInterface.Interact`
  (`self.K2_DestroyActor`)
  (`KismetSystemLibrary.PrintString` "Item Picked Up" true true (struct :`G` 1.0 :`B` 0.098495 :`A` 1.0))
  (bind _asthird_person_character (cast `/Game/ThirdPersonBP/Blueprints/ThirdPersonCharacter` (`GameplayStatics.GetPlayerCharacter` 0)))
  (set `/Game/ThirdPersonBP/Blueprints/ThirdPersonCharacter.HasKey` true _asthird_person_character))

(event `Show Prompt`
  (bind _asthird_person_character (cast `/Game/ThirdPersonBP/Blueprints/ThirdPersonCharacter` (`GameplayStatics.GetPlayerCharacter` 0)))
  (set `/Game/ThirdPersonBP/Blueprints/PlayerUI.InteractText` "Press E to pick up" (`/Game/ThirdPersonBP/Blueprints/ThirdPersonCharacter.Player UI` _asthird_person_character)))

(event `Hide Prompt`
  (bind _asthird_person_character (cast `/Game/ThirdPersonBP/Blueprints/ThirdPersonCharacter` (`GameplayStatics.GetPlayerCharacter` 0)))
  (set `/Game/ThirdPersonBP/Blueprints/PlayerUI.InteractText` "" (`/Game/ThirdPersonBP/Blueprints/ThirdPersonCharacter.Player UI` _asthird_person_character)))

(fn `UserConstructionScript`)